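; TripStability_BP keeps a running Stability score for what its name calls trip stability.
; Two custom events add positive points or subtract negative points, and each then calls SetStabilityEffect.
; SetStabilityEffect compares the score with zero and only prints Positive, Neutral or Negative, with no other effect applied.
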(event Custom|Stability--
  (params (Negative%20Points :type Float%20%28single-precision%29))
  (Variables|Default|Setstability (- (Variables|Default|Getstability) Negative%20Points))
  (CallFunction|SetStabilityEffect))

(event Custom|Stability++
  (params (Positive%20Points :type Float%20%28single-precision%29))
  (Variables|Default|Setstability (+ (Variables|Default|Getstability) Positive%20Points))
  (CallFunction|SetStabilityEffect))

(event Custom|Set%20Stability%20Effect
  (Math|Float|CompareFloat (Variables|Default|Getstability) 0.0
    (:>
      (Development|PrintString "Positive" true true "(R=0.000000,G=0.500000,B=1.000000,A=1.000000)"))
    (:==
      (Development|PrintString "Neutral" true true "(R=1.000000,G=1.000000,B=1.000000,A=1.000000)"))
    (:<
      (Development|PrintString "Negative" true true "(R=1.000000,G=0.050000,B=0.050000,A=1.000000)"))))

(fn ConstructionScript)