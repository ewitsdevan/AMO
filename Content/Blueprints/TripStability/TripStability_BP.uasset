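; TripStability_BP tracks a trip stability value that rises or falls through the ChangeStability event.
; Each change re-evaluates the effect and pushes the new value to the meter in TSWidget.
; SetStabilityEffect classifies the value as positive, neutral or negative, flagging "Closure" and "Ego Death" at the upper and lower thresholds.
; These effects are currently only printed strings, and the value is not clamped.
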(event Custom|Set%20Stability%20Effect
  (Math|Float|CompareFloat (Variables|Default|GetStability) 0.0
    (:>
      (Development|PrintString "Positive" true true "(R=0.000000,G=0.500000,B=1.000000,A=1.000000)")
      (Math|Float|CompareFloat (Variables|Default|GetStability) 5.0
        (:>
          _)
        (:==
          _))
      (Development|PrintString "Closure" true true "(R=0.000000,G=0.749020,B=1.000000,A=1.000000)"))
    (:==
      (Development|PrintString "Neutral" true true "(R=1.000000,G=1.000000,B=1.000000,A=1.000000)"))
    (:<
      (Development|PrintString "Negative" true true "(R=1.000000,G=0.050000,B=0.050000,A=1.000000)")
      (Math|Float|CompareFloat (Variables|Default|GetStability) -5.0
        (:==
          _)
        (:<
          _))
      (Development|PrintString "Ego Death" true true "(R=1.000000,G=0.098039,B=0.098039,A=1.000000)"))))

(event Custom|Change%20Stability
  (params (isNegative :type Boolean) (Value :type Float%20%28single-precision%29))
  (bind _ts_widget (Variables|Default|GetTS_Widget))
  (bind _meter (Variables|/Game/Blueprints/TripStability/TripStabilityTest_WBP.TripStabilityTest_WBP_C|GetMeter _ts_widget))
  (if isNegative
    (bind _output_get (Variables|Default|SetStability (- (Variables|Default|GetStability) Value)))
    (CallFunction|SetStabilityEffect)
    (Class|Slider|SetValue _meter _output_get)
    (else
      (bind _output_get_2 (Variables|Default|SetStability (+ (Variables|Default|GetStability) Value)))
      (CallFunction|SetStabilityEffect)
      (Class|Slider|SetValue _meter _output_get_2))))

(fn ConstructionScript)