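; Interior door Blueprint for modular houses, with a trigger volume intended for press-E interaction.
; Trigger overlap enables input from the first player controller and prints a prompt; leaving disables input.
; A Timeline-driven yaw swing that toggles the door open and closed by an IsClosed flag is present, but no event runs it.
; The Construction Script applies a configurable material to the door mesh.
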(event OnComponentEndOverlap(Trigger)
  (params (OverlappedComponent :type Primitive%20Component%20Object%20Reference) (OtherActor :type Actor%20Object%20Reference) (OtherComp :type Primitive%20Component%20Object%20Reference) (OtherBodyIndex :type Integer))
  (Input|DisableInput (Game|GetPlayerController 0)))

(event OnComponentBeginOverlap(Trigger)
  (params (OverlappedComponent :type Primitive%20Component%20Object%20Reference) (OtherActor :type Actor%20Object%20Reference) (OtherComp :type Primitive%20Component%20Object%20Reference) (OtherBodyIndex :type Integer) (bFromSweep :type Boolean) (SweepResult :type Hit%20Result%20Structure%20%28by%20ref%29))
  (Input|EnableInput (Game|GetPlayerController 0))
  (Development|PrintText "Press E" true false "(R=1.000000,G=1.000000,B=1.000000,A=1.000000)" 1.0))

(event Input|KeyboardEvents|E
  (params (Key :type Key%20Structure :default "None")))

(fn ConstructionScript
  (Rendering|Material|SetMaterial (Variables|Default|GetDoor) 0 (Variables|Default|GetElement%200)))